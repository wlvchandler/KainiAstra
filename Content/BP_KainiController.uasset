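; BP_KainiController shows the mouse cursor and highlights the static mesh component beneath it.
; On BeginPlay it creates an outline material instance and an empty overlay mesh component.
; Each Tick, a Visibility cursor trace copies a newly hit mesh and its relative transform onto the overlay, applies the outline to slot 0 and prints debug text.
; A trace miss clears the overlay.
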(event `self.ReceiveBeginPlay`
  ;[1 1 1] UNUSED
  (set `PlayerController.bShowMouseCursor` true (`GameplayStatics.GetPlayerController` 0))
  (bind _returnvalue (`KismetMaterialLibrary.CreateDynamicMaterialInstance` "/Game/UI/ComponentHighlight.ComponentHighlight"))
  (set `self.OutlineMaterial` _returnvalue)
  (bind _returnvalue_2 (`AddComponent|NODE_AddStaticMeshComponent-0`))
  (set `self.HighlightedStaticMesh` _returnvalue_2))

(event `self.ReceiveTick`
  (params (DeltaSeconds :type "Float (single-precision)"))
  (bind _highlightedstaticmesh (`self.HighlightedStaticMesh`))
  (bind _outlinematerial (`self.OutlineMaterial`))
  (bind _highlightedstaticmesh_2 (`self.HighlightedStaticMesh`))
  (bind (_hitresult _returnvalue) (`self.GetHitResultUnderCursorByChannel` (`GameplayStatics.GetPlayerController` 0) "TraceTypeQuery1" true))
  ;[1 1 1] UNUSED
  (if _returnvalue
    (bind _asstatic_mesh_component (cast `StaticMeshComponent` (`.HitComponent` (`GameplayStatics.BreakHitResult` _hitresult))))
    (if (!= (`StaticMeshComponent.StaticMesh` _asstatic_mesh_component) (`StaticMeshComponent.StaticMesh` (`self.HighlightedStaticMesh`)))
      (`SceneComponent.K2_SetRelativeTransform` (`self.HighlightedStaticMesh`) (`SceneComponent.GetRelativeTransform` _asstatic_mesh_component) false false)
      (`StaticMeshComponent.SetStaticMesh` (`self.HighlightedStaticMesh`) (`StaticMeshComponent.StaticMesh` _asstatic_mesh_component))
      (`PrimitiveComponent.SetMaterial` _highlightedstaticmesh_2 0 _outlinematerial)
      (`KismetSystemLibrary.PrintText` (`|FormatText` "Setting {X} to {Y}" (`KismetSystemLibrary.GetDisplayName` _highlightedstaticmesh_2) (`KismetSystemLibrary.GetDisplayName` _outlinematerial))))
    (else
      (`/Engine/EditorBlueprintResources/StandardMacros.IsValid` (`StaticMeshComponent.StaticMesh` _highlightedstaticmesh)
        (:`Is Valid`
          (`StaticMeshComponent.SetStaticMesh` _highlightedstaticmesh null))))))

(fn `UserConstructionScript`)